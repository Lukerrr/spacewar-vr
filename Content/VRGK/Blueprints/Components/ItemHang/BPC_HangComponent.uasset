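; VR hang-point component that automatically holds one nearby grabbable item until a hand grabs it.
; While empty, it scans "grab"-tagged actors every Tick for the nearest free, ungrabbed, tag-matching hang item within HangRadius, measured to bounding-sphere edge.
; Hanging disables physics and attaches the actor, aligned by the item component's inverted relative transform.
; A bound grab event detaches it, restoring physics and collision.
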(event `self.ReceiveTick`
  (params (DeltaSeconds :type "Float (single-precision)"))
  (bind _result (`self.GetNearestHangItem`))
  (if (not (`self.HasHangedItem`))
    (`/Engine/EditorBlueprintResources/StandardMacros.IsValid` _result
      (:`Is Valid`
        (`self.HangItem` _result)))))

(event `OnItemGrabbed`
  (params (InteractionComp :type "/Game/VRGK/Blueprints/Components/HandInteraction/BPC_HandInteraction Object Reference"))
  (remove `/Game/VRGK/Blueprints/Components/HandInteraction/BPC_HandInteraction.OnGrab` InteractionComp (delegate `OnItemGrabbed`))
  (`self.ReleaseItem`))

(fn `CanAttachItem`
  (params (Item :type "/Game/VRGK/Blueprints/Components/ItemHang/BPC_HangItemComponent Object Reference"))
  (returns (bResult :type Boolean))
  (bind _returnvalue (`self.GetOwner` Item))
  (bind _itemtag (`self.ItemTag`))
  ;[1 1 1] Must be valid
  (`/Engine/EditorBlueprintResources/StandardMacros.IsValid` Item
    (:`Is Valid`
      ;[1 1 1] Must be not hanged
      (if (`/Game/VRGK/Blueprints/Components/ItemHang/BPC_HangItemComponent.IsHanged` Item)
        (return false)
        (else
          ;[1 1 1] Must have a valid tag
          (if (or (`self.ComponentHasTag` Item _itemtag) (== _itemtag "None"))
            ;[1 1 1] Must have mesh as root
            (cast `MeshComponent` (`Actor.RootComponent` _returnvalue)
              (:`then`
                ;[1 1 1] Must be not grabbed
                (for _array_element (`Actor.K2_GetComponentsByClass` _returnvalue "/Game/VRGK/Blueprints/Components/HandInteraction/BPC_HandInteraction.BPC_HandInteraction_C")
                  (if (`/Game/VRGK/Blueprints/Components/HandInteraction/BPC_HandInteraction.IsGrabbed` _array_element)
                    (return false)))
                (return true))
              (:`CastFailed`
                (return false)))
            (else
              (return false))))))
    (:`Is Not Valid`
      (return false))))

(fn `GetDistanceToItem`
  (params (Item :type "/Game/VRGK/Blueprints/Components/ItemHang/BPC_HangItemComponent Object Reference"))
  (returns (Distance :type "Float (double-precision)"))
  (bind (_origin _boxextent _sphereradius) (`KismetSystemLibrary.GetComponentBounds` (`Actor.RootComponent` (`self.GetOwner` Item))))
  ;[1 1 1] Get distance to item's root component sphere bounds
  (return (`KismetMathLibrary.FMax` (- (`KismetMathLibrary.Vector_Distance` _origin (`self.K2_GetComponentLocation`)) _sphereradius))))

(fn `GetHangedItem`
  (returns (Result :type "/Game/VRGK/Blueprints/Components/ItemHang/BPC_HangItemComponent Object Reference") (bValid :type Boolean))
  (for _array_element (`self.GetChildrenComponents` true)
    (bind _asbpc_hang_item_component (cast `/Game/VRGK/Blueprints/Components/ItemHang/BPC_HangItemComponent` _array_element))
    (return _asbpc_hang_item_component true))
  (return null false))

(fn `GetNearestHangItem`
  (returns (Result :type "/Game/VRGK/Blueprints/Components/ItemHang/BPC_HangItemComponent Object Reference"))
  (locals (MinDistance :type "Float (double-precision)" :default -1.0) (NearestItem :type "/Game/VRGK/Blueprints/Components/ItemHang/BPC_HangItemComponent Object Reference"))
  (bind _outactors (`GameplayStatics.GetAllActorsWithTag` "grab"))
  (for _array_element _outactors
    (bind _returnvalue (`Actor.GetComponentByClass` _array_element "/Game/VRGK/Blueprints/Components/ItemHang/BPC_HangItemComponent.BPC_HangItemComponent_C"))
    (if (`self.CanAttachItem` _returnvalue)
      (bind _distance (`self.GetDistanceToItem` _returnvalue))
      (if (or (not (`KismetSystemLibrary.IsValid` (`local.NearestItem`))) (< _distance (`local.MinDistance`)))
        (set `local.NearestItem` _returnvalue)
        (set `local.MinDistance` _distance))))
  (if (<= (`local.MinDistance`) (`self.HangRadius`))
    (return (`local.NearestItem`))
    (else
      (return null))))

(fn `HangItem`
  (params (Item :type "/Game/VRGK/Blueprints/Components/ItemHang/BPC_HangItemComponent Object Reference"))
  (bind _returnvalue (`self.GetOwner` Item))
  (if (not (`self.HasHangedItem`))
    (set `self.HangedItem` Item)
    (`|ExecutionSequence`
      (:`then_0`
        (bind _asmesh_component (cast `MeshComponent` (`Actor.RootComponent` _returnvalue)))
        (`PrimitiveComponent.SetSimulatePhysics` _asmesh_component false)
        (`PrimitiveComponent.SetCollisionEnabled` _asmesh_component "QueryOnly"))
      (:`then_1`
        (`Actor.K2_AttachToComponent` _returnvalue self "None" "SnapToTarget" "SnapToTarget" "SnapToTarget" true)
        (`Actor.K2_SetActorRelativeTransform` _returnvalue (`KismetMathLibrary.InvertTransform` (`self.GetRelativeTransform` Item)) false true))
      (:`then_2`
        (add `/Game/VRGK/Blueprints/Components/HandInteraction/BPC_HandInteraction.OnGrab` (`Actor.GetComponentByClass` _returnvalue "/Game/VRGK/Blueprints/Components/HandInteraction/BPC_HandInteraction.BPC_HandInteraction_C") (`|CreateDelegate` :!event `OnItemGrabbed`))
        (`/Game/VRGK/Blueprints/Components/ItemHang/BPC_HangItemComponent.OnHangedEvent` (`self.HangedItem`))))))

(fn `HasHangedItem`
  (returns (bResult :type Boolean))
  (return (`KismetSystemLibrary.IsValid` (`self.HangedItem`))))

(fn `ReleaseItem`
  (bind _returnvalue (`self.GetOwner` (`self.HangedItem`)))
  (if (`self.HasHangedItem`)
    (`|ExecutionSequence`
      (:`then_0`
        (bind _asmesh_component (cast `MeshComponent` (`Actor.RootComponent` _returnvalue)))
        (`PrimitiveComponent.SetSimulatePhysics` _asmesh_component true)
        (`PrimitiveComponent.SetCollisionEnabled` _asmesh_component "QueryAndPhysics"))
      (:`then_1`
        (`Actor.K2_DetachFromActor` _returnvalue "KeepWorld" "KeepWorld" "KeepWorld")
        (`/Game/VRGK/Blueprints/Components/ItemHang/BPC_HangItemComponent.OnUnhanged` (`self.HangedItem`))
        (set `self.HangedItem` null)))))