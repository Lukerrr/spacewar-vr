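; VRGK menu overlay actor that shows a 3D menu widget and a back button using depth-test-disabled materials, with both widgets tickable while paused.
; Each widget's render target, polled until valid, feeds a dynamic material on a background component that the construction script scales to the widget's draw size.
; The back button pops the menu's widget stack and is shown, with query collision, only while that stack is not empty.
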(event `self.ReceiveBeginPlay`
  (bind _returnvalue (`WidgetComponent.GetRenderTarget` (`self.MenuWidget`)))
  (bind _returnvalue_2 (`WidgetComponent.GetRenderTarget` (`self.BackWidget`)))
  (`self.UpdateBackButtonVisibility` false)
  (`|ExecutionSequence`
    (:`then_0`
      ;[1 1 1] Setup Menu Overlay
      (`PrimitiveComponent.SetMaterial` (`self.MenuWidget`) 0 "/Game/VRGK/Materials/Widget/MI_DepthTestDisabledWidget3D_TwoSidedTranslucent.MI_DepthTestDisabledWidget3D_TwoSidedTranslucent")
      (`ActorComponent.SetTickableWhenPaused` (`self.MenuWidget`) true)
      (bind _returnvalue_3 (`PrimitiveComponent.CreateDynamicMaterialInstance` (`self.MenuWidgetBackground`) 0 "/Game/VRGK/Materials/Widget/MI_DepthTestDisabledWidget3D_TwoSidedTranslucent_Background.MI_DepthTestDisabledWidget3D_TwoSidedTranslucent_Background" "None"))
      (set `self.BGMaterial` _returnvalue_3)
      (`/Engine/EditorBlueprintResources/StandardMacros.IsValid` _returnvalue :!label _label
        (:`Is Valid`
          (`/Engine/EditorBlueprintResources/StandardMacros.DoOnce` false
            (:`Completed`
              (`MaterialInstanceDynamic.SetTextureParameterValue` (`self.BGMaterial`) "SlateUI" _returnvalue)
              (bind _asbpw_menu_overlay_widget (cast `/Game/VRGK/Blueprints/Menu/BPW_MenuOverlayWidget` (`WidgetComponent.GetUserWidgetObject` (`self.MenuWidget`))))
              (bind _output_get (set `self.MenuOverlayWidget` _asbpw_menu_overlay_widget))
              (add `/Game/VRGK/Blueprints/Menu/BPW_MenuOverlayWidget.OnWidgetStackUpdate` _output_get (delegate `OnWidgetStackUpdate`))
              (`self.OnWidgetStackUpdate`))))
        (:`Is Not Valid`
          (`KismetSystemLibrary.Delay` 0.0)
          (goto _label))))
    (:`then_1`
      ;[1 1 1] Setup Back Button
      (`PrimitiveComponent.SetMaterial` (`self.BackWidget`) 0 "/Game/VRGK/Materials/Widget/MI_DepthTestDisabledWidget3D_TwoSidedTranslucent.MI_DepthTestDisabledWidget3D_TwoSidedTranslucent")
      (`ActorComponent.SetTickableWhenPaused` (`self.BackWidget`) true)
      (bind _returnvalue_4 (`PrimitiveComponent.CreateDynamicMaterialInstance` (`self.BackWidgetBackground`) 0 "/Game/VRGK/Materials/Widget/MI_DepthTestDisabledWidget3D_TwoSidedTranslucent_Background.MI_DepthTestDisabledWidget3D_TwoSidedTranslucent_Background" "None"))
      (set `self.BGBackMaterial` _returnvalue_4)
      (`/Engine/EditorBlueprintResources/StandardMacros.IsValid` _returnvalue_2 :!label _label_2
        (:`Is Valid`
          (`/Engine/EditorBlueprintResources/StandardMacros.DoOnce` false
            (:`Completed`
              (`MaterialInstanceDynamic.SetTextureParameterValue` (`self.BGBackMaterial`) "SlateUI" _returnvalue_2)
              (bind _asbpw_menu_overlay_back (cast `/Game/VRGK/Blueprints/Menu/BPW_MenuOverlayBack` (`WidgetComponent.GetUserWidgetObject` (`self.BackWidget`))))
              (add `/Game/VRGK/Blueprints/Menu/BPW_MenuOverlayBack.OnBackButtonClicked` _asbpw_menu_overlay_back (delegate `OnBackButtonClicked`)))))
        (:`Is Not Valid`
          (`KismetSystemLibrary.Delay` 0.0)
          (goto _label_2))))))

(event `OnWidgetStackUpdate`
  ;[1 1 1] Setup Menu Overlay
  (`self.UpdateBackButtonVisibility` (not (`.IsEmpty` (`/Game/VRGK/Blueprints/Menu/BPW_MenuOverlayWidget.GetWidgetStackCount` (`self.MenuOverlayWidget`))))))

(event `self.ReceiveTick`
  (params (DeltaSeconds :type "Float (single-precision)")))

(event `OnBackButtonClicked`
  ;[1 1 1] Setup Back Button
  (`/Game/VRGK/Blueprints/Menu/BPW_MenuOverlayWidget.PopWidget` (`self.MenuOverlayWidget`)))

(event `UpdateScaling`
  (params (BG :type "SceneComponent Object Reference") (Widget :type "WidgetComponent Object Reference"))
  (bind _relativescale3d_x (`KismetMathLibrary.BreakVector` (`SceneComponent.RelativeScale3D` Widget)))
  (bind (_returnvalue_x _returnvalue_y) (`KismetMathLibrary.BreakVector2D` (/ (* (`WidgetComponent.GetDrawSize` Widget) _relativescale3d_x) 100.0)))
  ;[1 1 1] Update Scaling of Widget
  (`SceneComponent.SetRelativeScale3D` BG (`KismetMathLibrary.MakeVector` _returnvalue_x _returnvalue_y _returnvalue_x)))

(event `UpdateBackButtonVisibility`
  (params (Visible :type Boolean))
  ;[1 1 1] Back Button Visibility
  (`SceneComponent.SetVisibility` (`self.BackWidget`) Visible false)
  (`SceneComponent.SetVisibility` (`self.BackWidgetBackground`) Visible false)
  (`PrimitiveComponent.SetCollisionEnabled` (`self.BackWidget`) (select `bool` Visible :`false` "NoCollision" :`true` "QueryOnly" :!type "ECollisionEnabled Enum")))

(fn `UserConstructionScript`
  (`|ExecutionSequence`
    (:`then_0`
      (`self.UpdateScaling` (`self.MenuWidgetBackground`) (`self.MenuWidget`)))
    (:`then_1`
      (`self.UpdateScaling` (`self.BackWidgetBackground`) (`self.BackWidget`)))))