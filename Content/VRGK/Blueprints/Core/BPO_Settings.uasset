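; Settings object for the VR game, covering audio, subtitles, vibration, spectator view, player calibration, movement and rotation.
; Setters write into PersistentSaveGame and fire event dispatchers for listeners to apply changes, while getters read the stored values.
; Init rebroadcasts saved audio volumes, resolved from keys to SoundClasses through AudioSettings, and saved custom console commands.
; The command map allows storing extra settings, with lookups falling back to the live console variable.
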(event `Init`
  ;[1 1 1] Init; Begin Play
  (`self.UpdateAllAudio`)
  (`self.ApplyAllCustomCommands`))

(event `ApplyAllCustomCommands`
  (bind _customcommands (`/Game/VRGK/Blueprints/Saves/BP_PersistentSaveGame.CustomCommands` (`self.PersistentSaveGame`)))
  ;[1 1 1] Custom Console Commands. Can be used to save additional Settings.
  (bind _keys (`BlueprintMapLibrary.Map_Keys` _customcommands))
  (for _array_element _keys
    (`self.ApplyCustomCommand` _array_element (`BlueprintMapLibrary.Map_Find` _customcommands _array_element))))

(event `SetCustomCommand`
  (params (Command :type String) (Value :type Integer))
  ;[1 1 1] Custom Console Commands. Can be used to save additional Settings.
  (`BlueprintMapLibrary.Map_Add` (`/Game/VRGK/Blueprints/Saves/BP_PersistentSaveGame.CustomCommands` (`self.PersistentSaveGame`)) Command Value)
  (`self.ApplyCustomCommand` Command Value))

(event `ApplyCustomCommand`
  (params (Command :type String) (Value :type Integer))
  ;[1 1 1] Custom Console Commands. Can be used to save additional Settings.
  (`self.OnCommandRequest` (`KismetStringLibrary.Concat_StrStr` Command " " (`KismetStringLibrary.Conv_IntToString` Value))))

(fn `GetAudioVolume`
  (params (Key :type Name))
  (returns (Volume :type "Float (double-precision)"))
  (bind (_value _returnvalue) (`BlueprintMapLibrary.Map_Find` (`/Game/VRGK/Blueprints/Saves/BP_PersistentSaveGame.AudioVolumeSettings` (`self.PersistentSaveGame`)) Key))
  (if _returnvalue
    (return _value)
    (else
      (return 1.0))))

(fn `GetCrouchClimbingEnabled`
  (returns (Enabled :type Boolean))
  (return (`/Game/VRGK/Blueprints/Saves/BP_PersistentSaveGame.CrouchClimbingEnabled` (`self.PersistentSaveGame`))))

(fn `GetCustomCommandValue`
  (params (Command :type String))
  (returns (Value :type Integer))
  (bind (_value _returnvalue) (`BlueprintMapLibrary.Map_Find` (`/Game/VRGK/Blueprints/Saves/BP_PersistentSaveGame.CustomCommands` (`self.PersistentSaveGame`)) Command))
  (if _returnvalue
    (return _value)
    (else
      (bind _returnvalue_2 (`KismetSystemLibrary.GetConsoleVariableIntValue` Command))
      (return _returnvalue_2))))

(fn `GetRotationOptions`
  (returns (RotationType :type "/Game/VRGK/Blueprints/Player/PlayerCore/Enum_VRRotationOption Enum") (RotationSpeed :type "Float (double-precision)"))
  (bind _persistentsavegame (`self.PersistentSaveGame`))
  (return (`/Game/VRGK/Blueprints/Saves/BP_PersistentSaveGame.RotationType` _persistentsavegame) (`KismetMathLibrary.Conv_IntToDouble` (`/Game/VRGK/Blueprints/Saves/BP_PersistentSaveGame.RotationSpeed` _persistentsavegame))))

(fn `GetSeatedPlayerHeight`
  (returns (SittingPlayerHeight :type "Float (double-precision)"))
  (return (`/Game/VRGK/Blueprints/Saves/BP_PersistentSaveGame.SeatedPlayerHeight` (`self.PersistentSaveGame`))))

(fn `GetSeatedPlayModeEnabled`
  (returns (Enabled :type Boolean))
  (return (`/Game/VRGK/Blueprints/Saves/BP_PersistentSaveGame.SeatedPlayModeEnabled` (`self.PersistentSaveGame`))))

(fn `GetSpectatorFOV`
  (returns (Value :type "Float (double-precision)"))
  (return (`/Game/VRGK/Blueprints/Saves/BP_PersistentSaveGame.SpectatorFOV` (`self.PersistentSaveGame`))))

(fn `GetSpectatorFPS`
  (returns (Value :type "Float (double-precision)"))
  (return (`/Game/VRGK/Blueprints/Saves/BP_PersistentSaveGame.SpectatorFPS` (`self.PersistentSaveGame`))))

(fn `GetSpectatorType`
  (returns (SpectatorType :type "/Game/VRGK/Blueprints/SpectatorCams/Enum_SpectatorType Enum"))
  (return (`/Game/VRGK/Blueprints/Saves/BP_PersistentSaveGame.SpectatorType` (`self.PersistentSaveGame`))))

(fn `GetStandingPlayerHeight`
  (returns (StandingPlayerHeight :type "Float (double-precision)"))
  (return (`/Game/VRGK/Blueprints/Saves/BP_PersistentSaveGame.StandingPlayerHeight` (`self.PersistentSaveGame`))))

(fn `GetSubtitlesEnabled`
  (returns (SubtitlesEnabled :type Boolean))
  (return (`/Game/VRGK/Blueprints/Saves/BP_PersistentSaveGame.SubtitlesEnabled` (`self.PersistentSaveGame`))))

(fn `GetVibrationEnabled`
  (returns (VibrationEnabeld :type Boolean))
  (return (`/Game/VRGK/Blueprints/Saves/BP_PersistentSaveGame.VibrationEnabeld` (`self.PersistentSaveGame`))))

(fn `GetVRMovementSource`
  (returns (`Current Movement Source` :type "/Game/VRGK/Blueprints/Player/PlayerCore/Enum_VRMovementSource Enum"))
  (return (`/Game/VRGK/Blueprints/Saves/BP_PersistentSaveGame.VRMovementSource` (`self.PersistentSaveGame`))))

(fn `GetWorldScaleAdjustmentEnabled`
  (returns (Enabled :type Boolean))
  (return (`/Game/VRGK/Blueprints/Saves/BP_PersistentSaveGame.WorldScaleAdjustmentEnabled` (`self.PersistentSaveGame`))))

(fn `Set Audio Volume`
  (params (Key :type Name) (Volume :type "Float (double-precision)"))
  (bind _volume (`local.Volume`))
  (bind (_value _returnvalue) (`BlueprintMapLibrary.Map_Find` (`self.AudioSettings`) Key))
  (if _returnvalue
    (`BlueprintMapLibrary.Map_Add` (`/Game/VRGK/Blueprints/Saves/BP_PersistentSaveGame.AudioVolumeSettings` (`self.PersistentSaveGame`)) (`local.Key`) _volume)
    (`self.UpdateAudioVolume` _value _volume)
    (else
      (`KismetSystemLibrary.PrintString` null (`KismetStringLibrary.Concat_StrStr` "BPO_Settings - Did not find Volume Key in \"Set Audio Volume\": " (`KismetStringLibrary.Conv_NameToString` Key))))))

(fn `SetCrouchClimbingEnabled`
  (params (Enabled :type Boolean))
  (bind _output_get (set `/Game/VRGK/Blueprints/Saves/BP_PersistentSaveGame.CrouchClimbingEnabled` Enabled (`self.PersistentSaveGame`)))
  (`self.OnCrouchClimbingEnabled` _output_get))

(fn `SetRotationOptions`
  (params (NewType :type "/Game/VRGK/Blueprints/Player/PlayerCore/Enum_VRRotationOption Enum" :default "NewEnumerator0") (NewSpeed :type "Float (double-precision)"))
  (bind _persistentsavegame (`self.PersistentSaveGame`))
  (bind _output_get (set `/Game/VRGK/Blueprints/Saves/BP_PersistentSaveGame.RotationType` NewType _persistentsavegame))
  (set `/Game/VRGK/Blueprints/Saves/BP_PersistentSaveGame.RotationSpeed` (`KismetMathLibrary.FTrunc` NewSpeed) _persistentsavegame)
  (`self.OnRotationOptionsChanged` _output_get NewSpeed))

(fn `SetSeatedPlayerHeight`
  (params (NewSittingHeight :type "Float (double-precision)"))
  (set `/Game/VRGK/Blueprints/Saves/BP_PersistentSaveGame.SeatedPlayerHeight` NewSittingHeight (`self.PersistentSaveGame`))
  (`self.OnPlayerCalibrationUpdate` self))

(fn `SetSeatedPlayModeEnabled`
  (params (Enabled :type Boolean))
  (set `/Game/VRGK/Blueprints/Saves/BP_PersistentSaveGame.SeatedPlayModeEnabled` Enabled (`self.PersistentSaveGame`))
  (`self.OnPlayerCalibrationUpdate` self))

(fn `SetSpectatorFOV`
  (params (FOV :type "Float (double-precision)"))
  (bind _output_get (set `/Game/VRGK/Blueprints/Saves/BP_PersistentSaveGame.SpectatorFOV` FOV (`self.PersistentSaveGame`)))
  (`self.OnSpectatorFOVChanged` _output_get))

(fn `SetSpectatorFPS`
  (params (FOV :type "Float (double-precision)"))
  (bind _output_get (set `/Game/VRGK/Blueprints/Saves/BP_PersistentSaveGame.SpectatorFPS` FOV (`self.PersistentSaveGame`)))
  (`self.OnSpectatorFPSChanged` _output_get))

(fn `SetSpectatorType`
  (params (SpectatorType :type "/Game/VRGK/Blueprints/SpectatorCams/Enum_SpectatorType Enum" :default "NewEnumerator0"))
  (bind _output_get (set `/Game/VRGK/Blueprints/Saves/BP_PersistentSaveGame.SpectatorType` SpectatorType (`self.PersistentSaveGame`)))
  (`self.OnSpectatorTypeChanged` _output_get))

(fn `SetStandingPlayerHeight`
  (params (NewHeight :type "Float (double-precision)"))
  (set `/Game/VRGK/Blueprints/Saves/BP_PersistentSaveGame.StandingPlayerHeight` NewHeight (`self.PersistentSaveGame`))
  (`self.OnPlayerCalibrationUpdate` self))

(fn `SetSubtitlesEnabled`
  (params (Enabled :type Boolean))
  (bind _output_get (set `/Game/VRGK/Blueprints/Saves/BP_PersistentSaveGame.SubtitlesEnabled` Enabled (`self.PersistentSaveGame`)))
  (`self.OnSubtitlesEnabled` _output_get))

(fn `SetVibrationEnabled`
  (params (Enabled :type Boolean))
  (bind _output_get (set `/Game/VRGK/Blueprints/Saves/BP_PersistentSaveGame.VibrationEnabeld` Enabled (`self.PersistentSaveGame`)))
  (`self.OnVibrationEnabled` _output_get))

(fn `SetVRMovementSource`
  (params (NewMovementSource :type "/Game/VRGK/Blueprints/Player/PlayerCore/Enum_VRMovementSource Enum" :default "NewEnumerator0"))
  (bind _output_get (set `/Game/VRGK/Blueprints/Saves/BP_PersistentSaveGame.VRMovementSource` NewMovementSource (`self.PersistentSaveGame`)))
  (`self.OnVRMovementSourceChange` _output_get))

(fn `SetWorldScaleAdjustmentEnabled`
  (params (Enabled :type Boolean))
  (set `/Game/VRGK/Blueprints/Saves/BP_PersistentSaveGame.WorldScaleAdjustmentEnabled` Enabled (`self.PersistentSaveGame`))
  (`self.OnPlayerCalibrationUpdate` self))

(fn `UpdateAllAudio`
  (bind _audiovolumesettings (`/Game/VRGK/Blueprints/Saves/BP_PersistentSaveGame.AudioVolumeSettings` (`self.PersistentSaveGame`)))
  (bind _keys (`BlueprintMapLibrary.Map_Keys` _audiovolumesettings))
  (for _array_element _keys
    (bind (_value _returnvalue) (`BlueprintMapLibrary.Map_Find` (`self.AudioSettings`) _array_element))
    (if _returnvalue
      (`self.UpdateAudioVolume` _value (`BlueprintMapLibrary.Map_Find` _audiovolumesettings _array_element)))))

(fn `UpdateAudioVolume`
  (params (`Sound Class` :type "SoundClass Object Reference") (Volume :type "Float (double-precision)"))
  (`self.OnAudioVolumeRequest` `Sound Class` Volume))