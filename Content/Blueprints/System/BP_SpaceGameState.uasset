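; Space game state that manages transitions between levels and counts destroyed targets.
; TransitToLevel ignores overlapping requests, fades out with a level sequence, then hands loading to BP_TransientPawn, optionally fading in for a loading screen.
; Finishing waits out a minimum transit time, spawns and possesses a gameplay or menu pawn at a random PlayerStart, then fades in.
; Startup binding, initial transit and default-actor cleanup are disconnected from BeginPlay.
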(event `self.ReceiveBeginPlay`)

(event `OnTransitFinished`
  (bind _returnvalue (- (`self.TransitMinTime`) (- (`self.GetServerWorldTimeSeconds`) (`self.TransitStartTime`))))
  ;[1 1 1] Commit finish transient after a minimum delay
  (if (> _returnvalue 0.0)
    (`KismetSystemLibrary.Delay` _returnvalue))
  (`self.OnEndTransitToLevel`))

(event `OnBeginTransitToLevel`
  (params (Level :type "/Game/Blueprints/Game/Character/TransientPawn/Enums/BPE_GameLevelType Enum" :default "NewEnumerator0") (bLoadingScreen :type Boolean))
  ;[1 1 1] Fade out from old level
  (bind (_outactor _returnvalue) (`LevelSequencePlayer.CreateLevelSequencePlayer` "/Game/Sequence/Transient/Seq_TransientFadeOut.Seq_TransientFadeOut" (make `MovieSceneSequencePlaybackSettings` true)))
  (`KismetSystemLibrary.Delay` (`TimeManagementBlueprintLibrary.Conv_QualifiedFrameTimeToSeconds` (`MovieSceneSequencePlayer.GetEndTime` _returnvalue)))
  ;[1 1 1] Possess transient pawn
  (set `self.TransitStartTime` (`self.GetServerWorldTimeSeconds`))
  (set `self.TransitMinTime` (select `bool` bLoadingScreen :`false` (`self.TransitMinTimeNoLoadingScr`) :`true` (`self.TransitMinTimeLoadingScr`)))
  (`/Game/Blueprints/Game/Character/TransientPawn/BP_TransientPawn.TransitToLevel` (`self.GetTransientPawn`) Level bLoadingScreen)
  (set `self.CurrentLevel` Level)
  (if bLoadingScreen
    ;[1 1 1] Fade in to transient level if loading screen is needed
    (`LevelSequencePlayer.CreateLevelSequencePlayer` "/Game/Sequence/Transient/Seq_TransientFadeIn.Seq_TransientFadeIn" (make `MovieSceneSequencePlaybackSettings` true))))

(event `OnEndTransitToLevel`
  (bind _gamemode (`self.GetSpaceGameMode`))
  ;[1 1 1] Fade out from transient level
  (bind (_outactor _returnvalue) (`LevelSequencePlayer.CreateLevelSequencePlayer` "/Game/Sequence/Transient/Seq_TransientFadeOut.Seq_TransientFadeOut" (make `MovieSceneSequencePlaybackSettings` true)))
  (`KismetSystemLibrary.Delay` (`TimeManagementBlueprintLibrary.Conv_QualifiedFrameTimeToSeconds` (`MovieSceneSequencePlayer.GetEndTime` _returnvalue)))
  ;[1 1 1] Spawn and possess game mode pawn
  (bind _outactors (`GameplayStatics.GetAllActorsOfClass` "/Script/Engine.PlayerStart"))
  (bind _outitem (`KismetArrayLibrary.Array_Random` _outactors))
  (bind _returnvalue_2 (`|SpawnActorFromClass` (select `bool` (`|EnumEquality` (`self.CurrentLevel`) "NewEnumerator2") :`false` (`/Game/Blueprints/System/GameMode/BP_SpaceGameMode.DefaultMenuPawnClass` _gamemode) :`true` (`GameModeBase.DefaultPawnClass` _gamemode) :!type "Actor Class Reference") (`self.GetTransform` _outitem) "AlwaysSpawn" "OverrideRootScale" _outitem null))
  (bind _aspawn (cast `Pawn` _returnvalue_2)
    (:`then`
      _)
    (:`CastFailed`
      _))
  (`Controller.Possess` (`GameplayStatics.GetPlayerController` 0) _aspawn)
  (`/Game/Blueprints/Game/Character/TransientPawn/BP_TransientPawn.OnUnpossessed` (`self.GetTransientPawn`))
  ;[1 1 1] Fade in to target level
  (bind (_outactor_2 _returnvalue_3) (`LevelSequencePlayer.CreateLevelSequencePlayer` "/Game/Sequence/Transient/Seq_TransientFadeIn.Seq_TransientFadeIn" (make `MovieSceneSequencePlaybackSettings` true)))
  (`KismetSystemLibrary.Delay` (`TimeManagementBlueprintLibrary.Conv_QualifiedFrameTimeToSeconds` (`MovieSceneSequencePlayer.GetEndTime` _returnvalue_3)))
  (set `self.bTravelingToLevel` false))

(fn `AddDestroyedTarget`
  (`/Engine/EditorBlueprintResources/StandardMacros.IncrementInt` (`self.NumTargetsDestroyed`)))

(fn `ClearGameStats`
  (set `self.NumTargetsDestroyed` 0))

(fn `GetSpaceGameMode`
  (returns (GameMode :type "/Game/Blueprints/System/GameMode/BP_SpaceGameMode Object Reference"))
  (bind _asbp_space_game_mode (cast `/Game/Blueprints/System/GameMode/BP_SpaceGameMode` (`GameplayStatics.GetGameMode`))
    (:`then`
      _)
    (:`CastFailed`
      _))
  (return _asbp_space_game_mode))

(fn `GetTransientPawn`
  (returns (Pawn :type "/Game/Blueprints/Game/Character/TransientPawn/BP_TransientPawn Object Reference"))
  (bind _returnvalue (`GameplayStatics.GetActorOfClass` "/Game/Blueprints/Game/Character/TransientPawn/BP_TransientPawn.BP_TransientPawn_C"))
  (return _returnvalue))

(fn `TransitToLevel`
  (params (Level :type "/Game/Blueprints/Game/Character/TransientPawn/Enums/BPE_GameLevelType Enum" :default "NewEnumerator0") (bLoadingScreen :type Boolean))
  (if (not (`self.bTravelingToLevel`))
    (set `self.bTravelingToLevel` true)
    (`self.OnBeginTransitToLevel` Level bLoadingScreen)))

(fn `UserConstructionScript`)