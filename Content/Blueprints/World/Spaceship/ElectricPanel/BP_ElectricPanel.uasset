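; Breakable spaceship electric panel that the player repairs by hitting it with a wrench.
; While broken, a self-rescheduling event replays spark sound and particles and a timeline-driven light flash at random intervals.
; Wrench hits, throttled by a cooldown, add velocity-scaled, capped repair progress until FixUp clears the broken state and fires OnFixed.
; Mesh outline toggling in Break and FixUp is disconnected.
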(event `OnSparkEvent`
  (bind _sparkingdelay (`self.SparkingDelay`))
  (if (`self.bBroken`)
    (`AudioComponent.Play` (`self.SC_ElectricPanel_Sparks`) 0.0)
    (`ActorComponent.Activate` (`self.Sparks`) false)
    (`|ExecutionSequence`
      (:`then_0`
        (bind (_direction _intensity) (`Timeline|TL_Flashing` :!via `PlayFromStart`)
          (:`Update`
            (`LightComponent.SetIntensity` (`self.PointLight`) _intensity))))
      (:`then_1`
        (`KismetSystemLibrary.Delay` (`KismetMathLibrary.RandomFloatInRange` (`.Value` (break `FloatRangeBound` (break `FloatRange` _sparkingdelay))) (`.Value` (break `FloatRangeBound` (`.UpperBound` (break `FloatRange` _sparkingdelay))))))
        (`self.OnSparkEvent`)))))

(event `OnWrenchHit`
  (params (Velocity :type "Float (double-precision)") (Point :type "Vector Structure"))
  (bind _returnvalue (* Velocity (`self.PercentPerImpulse`)))
  (if (and (`self.IsBroken`) (`self.bCanHitByWrench`))
    (if (>= _returnvalue 0.0)
      (set `self.bCanHitByWrench` false)
      (`self.OnAddFixPercent` _returnvalue)
      (`GameplayStatics.SpawnSoundAtLocation` "/Game/Audio/SFX/Legacy/Wrench/SC_WrenchHitPanel.SC_WrenchHitPanel" Point (struct) 0.4 1.0 0.0 null null)
      (`KismetSystemLibrary.Delay` (`self.WrenchHitDelay`))
      (set `self.bCanHitByWrench` true))))

(event `OnAddFixPercent`
  (params (Percent :type "Float (double-precision)"))
  (bind _output_get (set `self.FixPercent` (`KismetMathLibrary.FMin` (+ (`self.FixPercent`) (`KismetMathLibrary.FMin` Percent 50.0)) 100.0)))
  (if (>= _output_get 100.0)
    (`self.FixUp`)))

(fn `Break`
  (if (not (`self.bBroken`))
    (set `self.bBroken` true)
    (set `self.FixPercent` 0.0)
    (`self.OnSparkEvent`)))

(fn `FixUp`
  (if (`self.bBroken`)
    (set `self.bBroken` false)
    (`self.OnFixed`)))

(fn `IsBroken`
  (returns (bBroken :type Boolean))
  (return (`self.bBroken`)))

(fn `UserConstructionScript`)