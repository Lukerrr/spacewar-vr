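; Spaceship controller that tracks ship health and drives the power-outage and repair loop.
; Damage cuts power and breaks randomly chosen electric panels, more as health drops; fixing all broken panels restores power.
; Power changes swap streamed normal/no-power levels, toggle soundtrack and notify BPI_ElectricDevice actors.
; At zero health it plays alarms at BP_AlarmPoint locations and transitions level through BP_SpaceGameState; debug keys test damage and lights.
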(event Custom|OnSpaceshipDamage
  ;[1 1 1] Damage events
  (CallFunction|DisableLights))

(event Custom|DisableLights
  (bind _electricpanels (LightsSystem|GetFixedElectricPanels))
  (bind _numpanels (LightsSystem|GetNumPanelstoBreak))
  (bind _returnvalue (Utilities|Array|Length _electricpanels))
  (bind _returnvalue_2 (Math|Integer|Min(Integer) _returnvalue _numpanels))
  ;[1 1 1] Lights system
  (if (Variables|LightsSystem|GetbLightsEnabled)
    (Utilities|FlowControl|Sequence
      (:then_0
        (LightsSystem|SetLightsEnabled false)
        (CallFunction|OnDisableLights))
      (:then_1
        ;;[1 1 1] Break electric panels on lights off
        (for _index (range 0 (- _returnvalue_2 1))
          (Default|Break (Utilities|Array|Get(acopy) _electricpanels _index)))
        (Variables|LightsSystem|SetNumElectricPanelsBroken (+ (Variables|LightsSystem|GetNumElectricPanelsBroken) _returnvalue_2))))))

(event Custom|EnableLights
  ;[1 1 1] Lights system
  (if (not (Variables|LightsSystem|GetbLightsEnabled))
    (LightsSystem|SetLightsEnabled true)
    (CallFunction|OnEnableLights)))

(event Custom|OnSpaceshipDestroyed
  ;[1 1 1] Damage events
  (AlarmSystem|PlayAlarmSound "/Game/Audio/SFX/Legacy/SpaceshipController/S_SpaceshipDestroyedAlarm.S_SpaceshipDestroyedAlarm")
  (bind _asbp_space_game_state (Utilities|Casting|CastToBP_SpaceGameState (Game|GetGameState))
    (:then
      _)
    (:CastFailed
      _))
  (Default|TransittoLevel _asbp_space_game_state "NewEnumerator4" false))

(event Custom|OnElectricPanelFixed_Event
  ;[1 1 1] Begin play
  ;;[1 1 1] Electric panels fix
  (bind _result (Math|Integer|DecrementInt (Variables|LightsSystem|GetNumElectricPanelsBroken))
    (:%20%20
      (if (<= _result 0)
        (Variables|LightsSystem|SetNumElectricPanelsBroken 0)
        (CallFunction|EnableLights)))))

(event Custom|CustomEvent)

(event Custom|CustomEvent_1)

(event Custom|OnEnableLights
  ;[1 1 1] Lights system
  (Class|GameplayStatics|LoadStreamLevelbySoftObjectPtr "/Game/Maps/Main/PLS_Normal.PLS_Normal" false false)
  (Utilities|FlowControl|Sequence
    (:then_0
      (Class|GameplayStatics|LoadStreamLevelbySoftObjectPtr "/Game/Maps/Main/PLS_Normal.PLS_Normal" true false))
    (:then_1
      (Class|GameplayStatics|UnloadStreamLevelbySoftObjectPtr "/Game/Maps/Main/PLS_NoPower.PLS_NoPower" false))))

(event Custom|OnDisableLights
  ;[1 1 1] Lights system
  (Class|GameplayStatics|LoadStreamLevelbySoftObjectPtr "/Game/Maps/Main/PLS_NoPower.PLS_NoPower" false false)
  (Utilities|FlowControl|Sequence
    (:then_0
      (Class|GameplayStatics|LoadStreamLevelbySoftObjectPtr "/Game/Maps/Main/PLS_NoPower.PLS_NoPower" true false))
    (:then_1
      (Class|GameplayStatics|UnloadStreamLevelbySoftObjectPtr "/Game/Maps/Main/PLS_Normal.PLS_Normal" false))))

(event EventBeginPlay
  ;[1 1 1] Begin play
  (CallFunction|OnEnableLights)
  (bind _asbp_space_game_state (Utilities|Casting|CastToBP_SpaceGameState (Game|GetGameState)))
  (Default|ClearGameStats _asbp_space_game_state)
  (bind _outactors (Actor|GetAllActorsOfClass "/Game/Blueprints/World/Spaceship/ElectricPanel/BP_ElectricPanel.BP_ElectricPanel_C"))
  (for _array_element _outactors
    (EventDispatchers|AssignOnFixed _array_element (delegate Custom|OnElectricPanelFixed_Event))))

(event Input|KeyboardEvents|DebugKeyY
  (params (Key :type Key%20Structure :default "None") (ActionValue :type Input%20Action%20Value%20Structure))
  ;[1 1 1] Debug
  (:Pressed
    (Utilities|FlowControl|FlipFlop
      (:A
        (CallFunction|DisableLights))
      (:B
        (CallFunction|EnableLights)))))

(event Input|KeyboardEvents|DebugKeyT
  (params (Key :type Key%20Structure :default "None") (ActionValue :type Input%20Action%20Value%20Structure))
  ;[1 1 1] Debug
  (:Pressed
    (DamageSystem|DamageSpaceship 4e+01)))

(fn ConstructionScript)

(fn DamageSpaceship
  (params (Damage :type Float%20%28double-precision%29))
  (if (> (Variables|DamageSystem|GetSpaceshipStatus) 0.0)
    (CallFunction|DisableLights)
    (bind _output_get (Variables|DamageSystem|SetSpaceshipStatus (Math|Float|Max(Float) (- (Variables|DamageSystem|GetSpaceshipStatus) Damage) 0.0)))
    (if (<= _output_get 0.0)
      (CallFunction|OnSpaceshipDestroyed))))

(fn GetSpaceshipStatus
  (return (Variables|DamageSystem|GetSpaceshipStatus)))

(fn SetLightsEnabled
  (params (bLightsEnabled :type Boolean))
  (bind _soundtrack (Variables|Default|GetSoundtrack))
  (bind _output_get (Variables|LightsSystem|SetbLightsEnabled bLightsEnabled))
  (Utilities|FlowControl|Sequence
    (:then_0
      (Audio|PlaySound2D (select _output_get "/Game/Audio/SFX/Legacy/SpaceshipController/SC_LightOn.SC_LightOn" "/Game/Audio/SFX/Legacy/SpaceshipController/SC_LightOff.SC_LightOff") 1.0 1.0 0.0 0 self)
      (if _output_get
        (Audio|Components|Audio|FadeIn _soundtrack 0.25 1.0 0.0 "Linear" :!class /Script/Engine.AudioComponent)
        (else
          (Audio|Components|Audio|StopDelayed _soundtrack 0.05))))
    (:then_1
      (bind _outactors (Actor|GetAllActorswithInterface "/Game/Blueprints/World/Spaceship/ElectricDevice/BPI_ElectricDevice.BPI_ElectricDevice_C"))
      (for _array_element _outactors
        (if _output_get
          (Class|BPIElectricDevice|Poweron(Message) _array_element)
          (else
            (Class|BPIElectricDevice|PowerOff(Message) _array_element)))))))

(fn GetFixedElectricPanels
  (bind _outactors (Actor|GetAllActorsOfClass "/Game/Blueprints/World/Spaceship/ElectricPanel/BP_ElectricPanel.BP_ElectricPanel_C"))
  (for _array_element _outactors
    (if (not (Default|IsBroken _array_element))
      (Utilities|Array|Add (LocalVariables|GetResult) _array_element)))
  (Utilities|Array|Shuffle (LocalVariables|GetResult))
  (return (LocalVariables|GetResult)))

(fn GetNumPanelstoBreak
  (bind _spaceshipstatus (Variables|DamageSystem|GetSpaceshipStatus))
  (if (< _spaceshipstatus 8e+01)
    (if (< _spaceshipstatus 4e+01)
      (return 3)
      (else
        (return 2)))
    (else
      (return 1))))

(fn GetAlarmPoints
  (bind _outactors (Actor|GetAllActorsOfClass "/Game/Blueprints/World/Spaceship/SpaceshipController/Alarms/BP_AlarmPoint.BP_AlarmPoint_C"))
  (for _array_element _outactors
    (Utilities|Array|Add (LocalVariables|GetResultPoints) (Transformation|GetActorLocation _array_element)))
  (return (LocalVariables|GetResultPoints)))

(fn PlayAlarmSound
  (params (Sound :type Sound%20Base%20Object%20Reference))
  (for _array_element (AlarmSystem|GetAlarmPoints)
    (bind _returnvalue (Audio|SpawnSoundatLocation Sound _array_element "0, 0, 0" 1.0 1.0 0.0 "/Game/Audio/SoundAttenuations/SA_Main.SA_Main" 0))
    (Audio|Components|Audio|Play _returnvalue 0.0)))