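; Spaceship beam cannon that, while powered, aims at the BP_SpaceshipCannonLocator, recharges and can fire at full charge to hit asteroids.
; Tick drives clamped yaw/pitch aiming with motor sounds, charging and interpolated barrel recoil.
; Firing uses timelines to stretch and retract the Niagara beam, sweeping sphere traces along its advancing tip.
; After each shot, a roll weighted by spaceship status may cut the ship's lights partway through recharging.
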(event Custom|OnStartFire
  ;[1 1 1] Weapon events
  (Components|Activation|Activate (Variables|Default|GetShootParticles) true)
  (Audio|Components|Audio|Play (Variables|Default|GetShootAudio) 0.0)
  (Utilities|FlowControl|RetriggerableDelay 0.5)
  (CallFunction|OnActivateRay)
  (Utilities|FlowControl|RetriggerableDelay (+ (Ammo|GetTravelDuration) (Variables|Ammo|GetRayLifetime)))
  (CallFunction|OnDeactivateRay))

(event Custom|OnActivateRay
  ;[1 1 1] Weapon events
  (Components|Activation|Activate (Variables|Default|GetBeamParticles) true)
  (Audio|Components|Audio|Stop (Variables|Default|GetTL_RayFadeOut))
  (Components|Timeline|PlayfromStart (Variables|Default|GetTL_RayMovement))
  (Camera|PlayWorldCameraShake "/Game/Blueprints/World/Spaceship/Cannon/Misc/BP_StartFireCameraShake.BP_StartFireCameraShake_C" (Transformation|GetWorldLocation (Variables|Default|GetBarrel)) 2e+03 1e+04))

(event Custom|OnDeactivateRay
  ;[1 1 1] Weapon events
  (Components|Timeline|PlayfromStart (Variables|Default|GetTL_RayFadeOut))
  (Components|Timeline|PlayfromStart (Variables|Default|GetTL_BarrelRecoil_End))
  ;;[1 1 1] Enable charge
  (Variables|Weapon|SetWeaponChargeTarget 1e+02)
  (bind _unpowerchargepercent (Utilities|DicePowerFailure))
  (Variables|Power|SetUnpowerChargePercent _unpowerchargepercent)
  (Camera|PlayWorldCameraShake "/Game/Blueprints/World/Spaceship/Cannon/Misc/BP_StopFireCameraShake.BP_StopFireCameraShake_C" (Transformation|GetWorldLocation (Variables|Default|GetBarrel)) 2e+03 1e+04))

(event Custom|OnColliderHit
  (params (Result :type Hit%20Result%20Structure))
  ;[1 1 1] Ammo projectile hit event
  (bind _asbp_asteroid (Utilities|Casting|CastToBP_Asteroid (.hitactor Result)))
  (Default|ProcessHit _asbp_asteroid (.impactpoint Result) (Transformation|GetActorForwardVector)))

(event Custom|OnPitchAimingStopped
  ;[1 1 1] Aiming events
  (Audio|SpawnSoundatLocation "/Game/Audio/SFX/Legacy/SpaceshipCannon/Rotation/SC_Cannon_StopMove.SC_Cannon_StopMove" (Transformation|GetWorldLocation (Variables|Default|GetRotateAudioHead)) "0, 0, 0" 1.0 1.0 0.0 "/Game/Audio/SoundAttenuations/SA_Main.SA_Main" 0))

(event Custom|OnPitchAimingStarted
  ;[1 1 1] Aiming events
  (Audio|SpawnSoundatLocation "/Game/Audio/SFX/Legacy/SpaceshipCannon/Rotation/SC_Cannon_StartMove.SC_Cannon_StartMove" (Transformation|GetWorldLocation (Variables|Default|GetRotateAudioHead)) "0, 0, 0" 1.0 1.0 0.0 "/Game/Audio/SoundAttenuations/SA_Main.SA_Main" 0))

(event Custom|OnYawAimingStarted
  ;[1 1 1] Aiming events
  (Audio|SpawnSoundatLocation "/Game/Audio/SFX/Legacy/SpaceshipCannon/Rotation/SC_Cannon_StartMove.SC_Cannon_StartMove" (Transformation|GetWorldLocation (Variables|Default|GetRotateAudioBase)) "0, 0, 0" 1.0 1.0 0.0 "/Game/Audio/SoundAttenuations/SA_Main.SA_Main" 0))

(event Custom|OnYawAimingStopped
  ;[1 1 1] Aiming events
  (Audio|SpawnSoundatLocation "/Game/Audio/SFX/Legacy/SpaceshipCannon/Rotation/SC_Cannon_StopMove.SC_Cannon_StopMove" (Transformation|GetWorldLocation (Variables|Default|GetRotateAudioBase)) "0, 0, 0" 1.0 1.0 0.0 "/Game/Audio/SoundAttenuations/SA_Main.SA_Main" 0))

(event EventBeginPlay
  (|SetupAnimations)
  (|SetupParticles)
  (|SetupRotationSounds))

(event EventTick
  (params (DeltaSeconds :type Float%20%28single-precision%29))
  (|UpdateRotationSounds)
  (if (Variables|Power|GetbPowered)
    (|ProcessBarrelMovement)
    (|ProcessTargetLocation)
    (|ProcessAimMovement)
    (|ChargeWeapon)))

(event EventPowerOff
  (Variables|Power|SetbPowered false))

(event EventPoweron
  (Variables|Power|SetbPowered true))

(event Input|KeyboardEvents|DebugKeyX
  (params (Key :type Key%20Structure :default "None") (ActionValue :type Input%20Action%20Value%20Structure))
  ;[1 1 1] Debug
)

(event Input|KeyboardEvents|DebugKeyR
  (params (Key :type Key%20Structure :default "None") (ActionValue :type Input%20Action%20Value%20Structure))
  ;[1 1 1] Debug
)

(fn ConstructionScript)

(fn GetRayScale
  (params (UniformScale :type Float%20%28double-precision%29))
  (return (/ (* UniformScale (Variables|Ammo|GetRayLength)) (Variables|Ammo|GetRayDefaultLength))))

(fn GetTravelDuration
  (return (/ (Variables|Ammo|GetRayLength) (Variables|Ammo|GetRayVelocity))))

(fn StartFire
  (if (Weapon|CanFire)
    (Weapon|StopFire)
    (CallFunction|OnStartFire)
    (Components|Timeline|PlayfromStart (Variables|Default|GetTL_BarrelRecoil_Start))
    ;[1 1 1] Uncharge and disable charge
    (Variables|Weapon|SetWeaponCharge 0.0)
    (Variables|Weapon|SetWeaponChargeTarget 0.0)))

(fn StopFire
  (for _array_element (Utilities|Array|MakeArray (Variables|Default|GetShootParticles) (Variables|Default|GetBeamParticles))
    (Components|Activation|Deactivate _array_element))
  (Transformation|SetRelativeLocation (Variables|Default|GetBeamParticles) "0, 0, 0" false false)
  (Audio|Components|Audio|Stop (Variables|Default|GetTL_RayFadeOut))
  (Ammo|MoveCollider "0, 0, 0" false))

(fn MoveCollider
  (params (Location :type Vector) (bSweep :type Boolean))
  (bind _barrel (Variables|Default|GetBarrel))
  (bind _returnvalue (Transformation|GetWorldTransform _barrel))
  (if bSweep
    (bind (_outhit _returnvalue_2) (Collision|SphereTraceByChannel (Math|Transform|TransformLocation _returnvalue (Variables|Ammo|GetColliderLocation)) (Math|Transform|TransformLocation _returnvalue Location) 64.0 "TraceTypeQuery1" false 0 "None"))
    (if _returnvalue_2
      (CallFunction|OnColliderHit _outhit)))
  (Variables|Ammo|SetColliderLocation Location))

(fn GetBarrelPosition
  (return (.y (Variables|/Script/Engine.SceneComponent|GetRelativeLocation (Variables|Default|GetCannon_Barrel)))))

(fn SetBarrelPosition
  (params (Position :type Float%20%28double-precision%29))
  (bind _cannon_barrel (Variables|Default|GetCannon_Barrel))
  (bind _relativelocation (Variables|/Script/Engine.SceneComponent|GetRelativeLocation _cannon_barrel))
  (Transformation|SetRelativeLocation _cannon_barrel (Math|Vector|MakeVector (.x _relativelocation) Position (.z _relativelocation)) false false))

(fn GetAnglesforTarget
  (params (Target :type Vector))
  (bind _returnvalue (- Target ""))
  (bind _cannon_top (Variables|Default|GetCannon_Top))
  (bind _relativelocation (Variables|/Script/Engine.SceneComponent|GetRelativeLocation _cannon_top))
  (bind _returnvalue_2 (- Target _relativelocation))
  (Utilities|FlowControl|Sequence
    (:then_0
      (LocalVariables|SetYawAngle (Class|KismetMathLibrary|DegAtan2 (.y _returnvalue) (.x _returnvalue))))
    (:then_1
      (LocalVariables|SetPitchAngle (- 1.8e+02 (+ (Class|KismetMathLibrary|DegAcos (Math|Vector|DotProduct (Math|Vector|Normalize (- "" _relativelocation)) (Math|Vector|Normalize _returnvalue_2))) (Class|KismetMathLibrary|DegAcos (/ (.z (Variables|/Script/Engine.SceneComponent|GetRelativeLocation (Variables|Default|GetCannon_Barrel))) (Math|Vector|VectorLength _returnvalue_2)))))))
    (:then_2
      (return (LocalVariables|GetYawAngle) (LocalVariables|GetPitchAngle)))))

(fn GetTargetLocation
  (bind _returnvalue (Actor|GetActorOfClass "/Game/Blueprints/World/Spaceship/Cannon/Locator/BP_SpaceshipCannonLocator.BP_SpaceshipCannonLocator_C"))
  (Utilities|IsValid _returnvalue
    (:Is%20Valid
      (return (Math|Transform|InverseTransformLocation (Transformation|GetActorTransform) (Transformation|GetActorLocation _returnvalue)) true))
    (:Is%20Not%20Valid
      (return "0, 0, 0" false))))

(fn GetCannonRotation
  (return (Math|Rotator|MakeRotator 0.0 (.roll (Variables|/Script/Engine.SceneComponent|GetRelativeRotation (Variables|Default|GetCannon_Top))) (.yaw (Variables|/Script/Engine.SceneComponent|GetRelativeRotation (Variables|Default|GetCannon_Bottom))))))

(fn SetCannonRotation
  (params (Rotaion :type Rotator))
  (Utilities|FlowControl|Sequence
    (:then_0
      (Transformation|SetRelativeRotation (Variables|Default|GetCannon_Bottom) (Math|Rotator|MakeRotator 0.0 0.0 (.yaw Rotaion)) false false))
    (:then_1
      (Transformation|SetRelativeRotation (Variables|Default|GetCannon_Top) (Math|Rotator|MakeRotator (.pitch Rotaion) 0.0 0.0) false false))))

(fn GetCannonState
  (if (.bValid (Aim|GetTargetLocation))
    (if (or (Variables|Aim|GetbAimingYaw) (Variables|Aim|GetbAimingPitch))
      (return "NewEnumerator1")
      (else
        (return "NewEnumerator2")))
    (else
      (return "NewEnumerator0"))))

(fn CanFire
  (return (and (>= (Variables|Weapon|GetWeaponCharge) 1e+02) (Variables|Power|GetbPowered))))

(fn GetCharge
  (return (Variables|Weapon|GetWeaponCharge)))

(fn GetPowerFailureChance
  (return (Math|Float|Lerp (Variables|Power|GetPowerFailureChanceMax) (Variables|Power|GetPowerFailureChanceMin) (/ (Default|GetSpaceshipStatus (Variables|Power|GetSpaceshipController)) 1e+02))))