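; Ship radar warning screen actor that alerts when the periscope detects a nearby asteroid.
; On begin play it binds to the periscope's detected and lost nearest-asteroid events to show or hide its widget component.
; Every tick it pushes the nearest asteroid's distance and time into the BP_RadarWarningUi widget, fetched through a cast helper.
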(event `self.ReceiveTick`
  (params (DeltaSeconds :type "Float (single-precision)"))
  (bind _gui (`self.GetGui`))
  (bind (_asteroid _dist _time) (`/Game/Blueprints/Game/Character/Periscope/BP_PeriscopePawn.GetNearestAsteroid` (`self.Periscope`)))
  (`/Game/Blueprints/Widget/RadarWarning/BP_RadarWarningUi.SetDistance` _gui _dist)
  (`/Game/Blueprints/Widget/RadarWarning/BP_RadarWarningUi.SetTime` _gui _time))

(event `self.ReceiveBeginPlay`
  (bind _periscope (`self.Periscope`))
  (add `/Game/Blueprints/Game/Character/Periscope/BP_PeriscopePawn.OnDetectedNearestAsteroid` _periscope (delegate `OnDetectedNearestAsteroid_Event`))
  (add `/Game/Blueprints/Game/Character/Periscope/BP_PeriscopePawn.OnLostNearestAsteroid` _periscope (delegate `OnLostNearestAsteroid_Event`)))

(event `OnDetectedNearestAsteroid_Event`
  (`SceneComponent.SetVisibility` (`self.Widget`) true false))

(event `OnLostNearestAsteroid_Event`
  (`SceneComponent.SetVisibility` (`self.Widget`) false false))

(fn `GetGui`
  (returns (Gui :type "/Game/Blueprints/Widget/RadarWarning/BP_RadarWarningUi Object Reference"))
  (bind _asbp_radar_warning_ui (cast `/Game/Blueprints/Widget/RadarWarning/BP_RadarWarningUi` (`WidgetComponent.GetWidget` (`self.Widget`)))
    (:`then`
      _)
    (:`CastFailed`
      _))
  (return _asbp_radar_warning_ui))

(fn `UserConstructionScript`)