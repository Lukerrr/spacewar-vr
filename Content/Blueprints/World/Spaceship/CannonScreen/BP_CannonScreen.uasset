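; BP_CannonScreen is an in-world spaceship screen that displays the cannon's status through a BP_CannonUi widget.
; Every Tick it pushes the referenced Cannon's charge and aim state, plus the game state's destroyed-target count, into the UI.
; GetGui casts the widget component's widget to BP_CannonUi, and the power on and off events show or hide that component.
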(event `self.ReceiveTick`
  (params (DeltaSeconds :type "Float (single-precision)"))
  (bind _gui (`self.GetGui`))
  (bind _cannon (`self.Cannon`))
  (`/Game/Blueprints/Widget/Cannon/BP_CannonUi.SetTargetPowerLevel` _gui (`/Game/Blueprints/World/Spaceship/Cannon/BP_SpaceshipCannon.GetCharge` _cannon))
  (`/Game/Blueprints/Widget/Cannon/BP_CannonUi.SetCannonAimState` _gui (`/Game/Blueprints/World/Spaceship/Cannon/BP_SpaceshipCannon.GetCannonState` _cannon))
  (bind _asbp_space_game_state (cast `/Game/Blueprints/System/BP_SpaceGameState` (`GameplayStatics.GetGameState`)))
  (`/Game/Blueprints/Widget/Cannon/BP_CannonUi.SetTargetsCount` _gui (`/Game/Blueprints/System/BP_SpaceGameState.NumTargetsDestroyed` _asbp_space_game_state)))

(event `/Game/Blueprints/World/Spaceship/ElectricDevice/BPI_ElectricDevice.PowerOn`
  (`SceneComponent.SetVisibility` (`self.Widget`) true false))

(event `/Game/Blueprints/World/Spaceship/ElectricDevice/BPI_ElectricDevice.PowerOff`
  (`SceneComponent.SetVisibility` (`self.Widget`) false false))

(fn `GetGui`
  (returns (Gui :type "/Game/Blueprints/Widget/Cannon/BP_CannonUi Object Reference"))
  (bind _asbp_cannon_ui (cast `/Game/Blueprints/Widget/Cannon/BP_CannonUi` (`WidgetComponent.GetWidget` (`self.Widget`))))
  (return _asbp_cannon_ui))

(fn `UserConstructionScript`)