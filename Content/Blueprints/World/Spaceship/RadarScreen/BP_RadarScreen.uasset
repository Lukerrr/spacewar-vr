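; BP_RadarScreen is a spaceship radar screen that displays asteroids reported by a Periscope through a BP_RadarWidget on its Widget component.
; Every tick it passes the Periscope's radar range and asteroid positions to the widget.
; Positions become 2D offsets from the Periscope in world axes, ignoring height and rotation, with Y as horizontal and negated X as vertical.
; Poweron and PowerOff events show or hide the screen.
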(event `self.ReceiveTick`
  (params (DeltaSeconds :type "Float (single-precision)"))
  (bind _widget (`self.GetRadarWidget`))
  (`/Game/Blueprints/Widget/Radar/BP_RadarWidget.SetRadarRange` _widget (`/Game/Blueprints/Game/Character/Periscope/BP_PeriscopePawn.RadarRange` (`self.Periscope`)))
  (`/Game/Blueprints/Widget/Radar/BP_RadarWidget.SetAsteroids` _widget (`self.GetAsteroids2DPositions`)))

(event `/Game/Blueprints/World/Spaceship/ElectricDevice/BPI_ElectricDevice.PowerOn`
  (`SceneComponent.SetVisibility` (`self.Widget`) true false))

(event `/Game/Blueprints/World/Spaceship/ElectricDevice/BPI_ElectricDevice.PowerOff`
  (`SceneComponent.SetVisibility` (`self.Widget`) false false))

(fn `GetAsteroids2DPositions`
  (returns (Result :type "Array of Vector2D Structure"))
  (locals (AsteroidPositions :type "Array of Vector2D Structure"))
  (bind _periscope (`self.Periscope`))
  (for _array_element (`/Game/Blueprints/Game/Character/Periscope/BP_PeriscopePawn.GetAsteroids` _periscope)
    (bind (_returnvalue_x _returnvalue_y) (`KismetMathLibrary.BreakVector` (- (`/Game/Blueprints/World/Space/Asteroid/BP_Asteroid.GetAsteroidLocation` _array_element) (`self.K2_GetActorLocation` _periscope))))
    (`KismetArrayLibrary.Array_Add` (`local.AsteroidPositions`) (`KismetMathLibrary.MakeVector2D` _returnvalue_y (* _returnvalue_x -1.0))))
  (return (`local.AsteroidPositions`)))

(fn `GetRadarWidget`
  (returns (Widget :type "/Game/Blueprints/Widget/Radar/BP_RadarWidget Object Reference"))
  (bind _asbp_radar_widget (cast `/Game/Blueprints/Widget/Radar/BP_RadarWidget` (`WidgetComponent.GetWidget` (`self.Widget`))))
  (return _asbp_radar_widget))

(fn `UserConstructionScript`)