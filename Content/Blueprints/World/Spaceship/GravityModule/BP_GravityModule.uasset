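; BP_GravityModule is a spaceship world actor that pulls living asteroids toward itself.
; Every Tick it finds all BP_Asteroid actors and applies linear velocity to item 0 of each Geometry Collection, scaled by GravityAcceleration and delta time.
; The pull grows with distance up to the Sphere radius and stays at full strength beyond it, with no cutoff.
; A persistent field system node is present but never runs.
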(event `self.ReceiveBeginPlay`)

(event `self.ReceiveTick`
  (params (DeltaSeconds :type "Float (single-precision)"))
  (bind _returnvalue (`self.K2_GetActorLocation`))
  (bind _outactors (`GameplayStatics.GetAllActorsOfClass` "/Game/Blueprints/World/Space/Asteroid/BP_Asteroid.BP_Asteroid_C"))
  (for _array_element _outactors
    (if (`/Game/Blueprints/World/Space/Asteroid/BP_Asteroid.IsAlive` _array_element)
      (bind _location (`/Game/Blueprints/World/Space/Asteroid/BP_Asteroid.GetAsteroidLocation` _array_element))
      (`GeometryCollectionComponent.ApplyLinearVelocity` (`/Game/Blueprints/World/Space/Asteroid/BP_Asteroid.GeometryCollection` _array_element) 0 (* (`KismetMathLibrary.Normal` (- _returnvalue _location)) (* (`self.GravityAcceleration`) (`KismetMathLibrary.FClamp` (/ (`KismetMathLibrary.Vector_Distance` _location _returnvalue) (`self.GetGravityRadius`))) (`GameplayStatics.GetWorldDeltaSeconds`)))))))

(fn `GetGravityRadius`
  (returns (Radius :type "Float (double-precision)"))
  (return (`SphereComponent.SphereRadius` (`self.Sphere`))))

(fn `UserConstructionScript`)