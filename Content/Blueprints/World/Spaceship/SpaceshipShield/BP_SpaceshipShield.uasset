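; Spaceship shield actor that turns asteroid impacts into damage on the spaceship.
; A hit on its Box component by a live BP_Asteroid marks that asteroid dead, so it counts only once, and applies fixed damage through the SpaceshipController.
; Each counted impact also plays a sound and a world camera shake at the hit location.
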(event `self.Box.OnComponentHit`
  (params (HitComponent :type "PrimitiveComponent Object Reference") (OtherActor :type "Actor Object Reference") (OtherComp :type "PrimitiveComponent Object Reference") (NormalImpulse :type "Vector Structure") (Hit :type "HitResult Structure (by ref)"))
  (bind _asbp_asteroid (cast `/Game/Blueprints/World/Space/Asteroid/BP_Asteroid` OtherActor))
  (if (`/Game/Blueprints/World/Space/Asteroid/BP_Asteroid.IsAlive` _asbp_asteroid)
    (set `/Game/Blueprints/World/Space/Asteroid/BP_Asteroid.bAlive` false _asbp_asteroid)
    (`/Game/Blueprints/World/Spaceship/SpaceshipController/BP_SpaceshipController.DamageSpaceship` (`self.SpaceshipController`) 40.0)
    (bind _returnvalue (`GameplayStatics.SpawnSoundAtLocation` "/Game/Audio/SFX/Legacy/SpaceshipImpact/SC_SpaceshipImpact.SC_SpaceshipImpact" Hit_Location (struct) 1.0 1.0 0.0 null null))
    (`self.SetOwner` (`ActorComponent.GetOwner` _returnvalue) self)
    (`GameplayStatics.PlayWorldCameraShake` "/Game/Blueprints/World/Spaceship/SpaceshipShield/Misc/BP_SpaceshipImpactCameraShake.BP_SpaceshipImpactCameraShake_C" Hit_Location 20000.0 200000.0)))

(fn `UserConstructionScript`)