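; BP_SpaceshipStatusScreen is an in-world spaceship screen that displays the ship's current status through a widget component.
; Every tick it reads the status from SpaceshipController and sends it as the target status level to the BP_SpaceshipStatusUi widget, fetched by a cast in GetGui.
; Poweron and PowerOff events show and hide the widget component without propagating to its children.
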(event `self.ReceiveTick`
  (params (DeltaSeconds :type "Float (single-precision)"))
  (`/Game/Blueprints/Widget/SpaceshipStatus/BP_SpaceshipStatusUi.SetTargetStatusLevel` (`self.GetGui`) (`/Game/Blueprints/World/Spaceship/SpaceshipController/BP_SpaceshipController.GetSpaceshipStatus` (`self.SpaceshipController`))))

(event `/Game/Blueprints/World/Spaceship/ElectricDevice/BPI_ElectricDevice.PowerOn`
  (`SceneComponent.SetVisibility` (`self.Widget`) true false))

(event `/Game/Blueprints/World/Spaceship/ElectricDevice/BPI_ElectricDevice.PowerOff`
  (`SceneComponent.SetVisibility` (`self.Widget`) false false))

(fn `GetGui`
  (returns (Gui :type "/Game/Blueprints/Widget/SpaceshipStatus/BP_SpaceshipStatusUi Object Reference"))
  (bind _asbp_spaceship_status_ui (cast `/Game/Blueprints/Widget/SpaceshipStatus/BP_SpaceshipStatusUi` (`WidgetComponent.GetWidget` (`self.Widget`)))
    (:`then`
      _)
    (:`CastFailed`
      _))
  (return _asbp_spaceship_status_ui))

(fn `UserConstructionScript`)