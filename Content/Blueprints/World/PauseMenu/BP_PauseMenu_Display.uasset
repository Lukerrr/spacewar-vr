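; In-world pause menu display with main and settings screens, handling continue, settings navigation and exit through BP_SpaceGameState level transition.
; Timelines slide and fade screens, including swipes between General, Graphics and Audio settings.
; Query collision gates each screen's interaction and doubles as the settings-open state.
; Each animation holds a counted lock, so show or hide requests made meanwhile set flags that Tick applies later.
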(event `self.ReceiveBeginPlay`
  (for _array_element (`self.K2_GetComponentsByClass` "/Script/Engine.TimelineComponent")
    (`TimelineComponent.SetPlayRate` _array_element (`self.AnimationsRate`)))
  (set `self.SettingsScreens` (`|MakeArray` (`self.Settings_General`) (`self.Settings_Graphics`) (`self.Settings_Audio`)))
  (if (`self.IsActive`)
    (`self.EnablePauseDisplay`)))

(event `self.ReceiveTick`
  (params (DeltaSeconds :type "Float (single-precision)"))
  (if (`self.CanTogglePauseDisplay`)
    (`|ExecutionSequence`
      (:`then_0`
        (if (`self.bDisablePauseDisplayFlag`)
          (set `self.bDisablePauseDisplayFlag` false)
          (`self.DisablePauseDisplay`)))
      (:`then_1`
        (if (`self.bEnablePauseDisplayFlag`)
          (set `self.bEnablePauseDisplayFlag` false)
          (`self.EnablePauseDisplay`))))))

(event `OnShowPauseMenu`
  (`self.DoShowPauseMenu`))

(event `OnShowSettings`
  (`self.DoHidePauseMenu`)
  (`self.DoShowSettings`))

(event `OnHideSettings`
  (`self.DoHideSettings`))

(event `OnHidePauseMenu`
  (`self.DoHidePauseMenu`))

(event `OnExitSettings`
  (`self.DoHideSettings`)
  (`self.DoShowPauseMenu`))

(event `OnSettingsSwipe`
  (params (bLeft :type Boolean))
  (`self.SetScreenEnabled` (`self.Settings_Header`))
  (`self.SetScreenEnabled` (`self.GetActiveSettingsScreen`))
  (`self.PlayAnim` (select `bool` bLeft :`false` (`self.TL_Settings_SwipeRight`) :`true` (`self.TL_Settings_SwipeLeft`)))
  (`self.SetActiveSettingsScreen` (+ (`self.ActiveSettingsScreen`) (`KismetMathLibrary.SelectInt` 1 -1 bLeft)))
  (`self.PlayAnim` (select `bool` bLeft :`false` (`self.TL_Settings_SwipeLeft`) :`true` (`self.TL_Settings_SwipeRight`)) true)
  (`self.SetScreenEnabled` (`self.Settings_Header`) true))

(fn `CanTogglePauseDisplay`
  (returns (bResult :type Boolean))
  (return (<= (`self.DisplayToggleLock`) 0)))

(fn `DisablePauseDisplay`
  (if (`self.CanTogglePauseDisplay`)
    (if (`self.IsSettingsScreenOpened`)
      (`self.OnHideSettings`)
      (else
        (`self.OnHidePauseMenu`)))
    (set `self.IsActive` false)
    (else
      (set `self.bDisablePauseDisplayFlag` true))))

(fn `EnablePauseDisplay`
  (if (`self.CanTogglePauseDisplay`)
    (`self.OnShowPauseMenu`)
    (set `self.IsActive` true)
    (else
      (set `self.bEnablePauseDisplayFlag` true))))

(fn `GetActiveSettingsScreen`
  (returns (Screen :type "SensorWidgetComponent Object Reference"))
  (return (`|GetArrayItem` (`self.SettingsScreens`) (`self.ActiveSettingsScreen`))))

(fn `GetAnimationLength`
  (params (Timeline :type "TimelineComponent Object Reference"))
  (returns (Length :type "Float (double-precision)"))
  (return (+ (/ (`TimelineComponent.GetTimelineLength` Timeline) (`self.AnimationsRate`)) 0.05)))

(fn `IsSettingsScreenOpened`
  (returns (bOpened :type Boolean))
  (switch `ECollisionEnabled` (`PrimitiveComponent.GetCollisionEnabled` (`self.Settings_Header`))
    (:`NoCollision`
      (return false))
    (:`QueryOnly`
      _)
    (:`PhysicsOnly`
      _)
    (:`QueryAndPhysics`
      _)
    (:`ProbeOnly`
      _)
    (:`QueryAndProbe`
      _))
  (return true))

(fn `OnPauseContinue`
  (`self.DisablePauseDisplay`))

(fn `OnPauseEnterSettings`
  (`self.SetActiveSettingsScreen` (`self.DefaultActiveSettingsScreen`))
  (`self.OnShowSettings`))

(fn `OnPauseExit`
  (`self.OnHidePauseMenu`)
  (bind _asbp_space_game_state (cast `/Game/Blueprints/System/BP_SpaceGameState` (`GameplayStatics.GetGameState`)))
  (`/Game/Blueprints/System/BP_SpaceGameState.TransitToLevel` _asbp_space_game_state "NewEnumerator1" true))

(fn `OnPauseExitSettings`
  (`self.OnExitSettings`))

(fn `OnPauseSettingsListLeft`
  (`self.OnSettingsSwipe` true))

(fn `OnPauseSettingsListRight`
  (`self.OnSettingsSwipe` false))

(fn `SetActiveSettingsScreen`
  (params (ScreenNumber :type Integer))
  (bind _returnvalue (- (`KismetArrayLibrary.Array_Length` (`self.SettingsScreens`)) 1))
  (bind _output_get (set `self.ActiveSettingsScreen` (`KismetMathLibrary.Clamp` ScreenNumber 0 _returnvalue)))
  (bind _aswidget_pallet_settings_pause_header (cast `/Game/ThirdParty/AFCore/Blueprints/Widgets/Pallets/Settings/Widget_Pallet_Settings_Pause_Header` (`WidgetComponent.GetUserWidgetObject` (`self.Settings_Header`))))
  (`/Game/ThirdParty/AFCore/Blueprints/Widgets/Pallets/Settings/Widget_Pallet_Settings_Pause_Header.OnActiveSettingsScreenChanged` _aswidget_pallet_settings_pause_header _output_get _returnvalue))

(fn `SetScreenEnabled`
  (params (Screen :type "SensorWidgetComponent Object Reference") (bEnabled :type Boolean))
  (`PrimitiveComponent.SetCollisionEnabled` Screen (select `bool` bEnabled :`false` "NoCollision" :`true` "QueryOnly" :!type "ECollisionEnabled Enum")))

(fn `TogglePauseMenu`
  (if (`self.IsActive`)
    (`self.DisablePauseDisplay`)
    (else
      (`self.EnablePauseDisplay`))))

(fn `UserConstructionScript`)