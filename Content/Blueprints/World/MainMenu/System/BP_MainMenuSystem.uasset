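; BP_MainMenuSystem is the main menu actor that turns button presses into sequence playback for starting the game, exiting, and opening or closing settings.
; Each button handler plays its matching sequence through that sequence's SequencePlayer.
; IsInteractable gates every handler, ignoring presses while any of the four sequences is still playing.
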(fn `IsInteractable`
  (returns (bInteractable :type Boolean))
  (for _array_element (`|MakeArray` (`self.GameStartSequence`) (`self.OpenSettingsSequence`) (`self.CloseSettingsSequence`) (`self.GameExitSequence`))
    (if (`MovieSceneSequencePlayer.IsPlaying` (`LevelSequenceActor.SequencePlayer` _array_element))
      (return false)))
  (return true))

(fn `OnCloseSettingsButtonPressed`
  (if (`self.IsInteractable`)
    (`MovieSceneSequencePlayer.Play` (`LevelSequenceActor.SequencePlayer` (`self.CloseSettingsSequence`)))))

(fn `OnExitButtonPressed`
  (if (`self.IsInteractable`)
    (`MovieSceneSequencePlayer.Play` (`LevelSequenceActor.SequencePlayer` (`self.GameExitSequence`)))))

(fn `OnOpenSettingsButtonPressed`
  (if (`self.IsInteractable`)
    (`MovieSceneSequencePlayer.Play` (`LevelSequenceActor.SequencePlayer` (`self.OpenSettingsSequence`)))))

(fn `OnStartButtonPressed`
  (if (`self.IsInteractable`)
    (`MovieSceneSequencePlayer.Play` (`LevelSequenceActor.SequencePlayer` (`self.GameStartSequence`)))))

(fn `UserConstructionScript`)