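; Destructible space asteroid built on a Chaos Geometry Collection that drifts and spins from preset start velocities.
; ProcessHit projects the hit inward along the shot direction, then Explode counts the destroyed target in the game state and frees radar aiming traces.
; After a short delay, radial strain and culled velocity fields shatter and scatter it.
; Size-scaled particles, sound and an emission timeline for the dynamic material's glow accompany the blast.
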(event `self.ReceiveBeginPlay`
  (bind _geometrycollection (`self.GeometryCollection`))
  (bind _geometrycollection_2 (`self.GeometryCollection`))
  (bind _returnvalue (`KismetMaterialLibrary.CreateDynamicMaterialInstance` "/Game/ThirdParty/Asteroids_Planet/Materials/Asteroids/MI_Asteroid_07.MI_Asteroid_07"))
  (bind _output_get (set `self.AsteroidMaterial` _returnvalue))
  (`PrimitiveComponent.SetMaterial` _geometrycollection 0 _output_get)
  (`PrimitiveComponent.SetMaterial` _geometrycollection 1 _output_get)
  (`NiagaraComponent.SetVariableFloat` (`self.ExplosionParticles`) "User.Scale" (/ (`self.GetExplosionRadius` 1.0) 100.0))
  (`|ExecutionSequence`
    (:`then_0`
      (`GeometryCollectionComponent.ApplyLinearVelocity` _geometrycollection_2 0 (`self.StartVelocityL`)))
    (:`then_1`
      (`GeometryCollectionComponent.ApplyAngularVelocity` _geometrycollection_2 0 (`self.StartVelocityA`)))))

(event `OnAsteroidExplode`
  (params (Center :type "Vector Structure") (Direction :type "Vector Structure"))
  (bind _fieldsystem (`self.FieldSystem`))
  (bind _returnvalue (`RadialFalloff.SetRadialFalloff` (`self.RadialFalloff`) (`self.GetExplosionMagnitude`) 0.0 1.0 0.0 (`self.GetExplosionRadius` 1.5) Center "Field_Falloff_Linear"))
  ;[1 1 1] Explosion event
  ;;[1 1 1] Fracture mesh
  (`KismetSystemLibrary.Delay` 0.075)
  (`FieldSystemComponent.ApplyPhysicsField` _fieldsystem true "Field_ExternalClusterStrain" null _returnvalue)
  (`FieldSystemComponent.ApplyPhysicsField` _fieldsystem true "Field_LinearVelocity" null (`CullingField.SetCullingField` (`self.CullingField`) _returnvalue (`RadialVector.SetRadialVector` (`self.RadialVector`) (`self.ExplosionForce`) Center) "Field_Culling_Outside"))
  (`GameplayStatics.SpawnSoundAtLocation` "/Game/Audio/SFX/Legacy/Asteroid/SC_AsteroidExplosion.SC_AsteroidExplosion" (`self.GetAsteroidLocation`) (struct) 1.0 1.0 0.0 null null))

(event `self.GeometryCollection.OnChaosBreakEvent`
  (params (BreakEvent :type "ChaosBreakEvent Structure (by ref)"))
  (if (`self.bAlive`)
    (set `self.bAlive` false)))

(fn `Explode`
  (params (Location :type "Vector Structure") (Direction :type "Vector Structure"))
  (bind _explosionparticles (`self.ExplosionParticles`))
  (if (`self.bAlive`)
    (bind _asbp_space_game_state (cast `/Game/Blueprints/System/BP_SpaceGameState` (`GameplayStatics.GetGameState`))
      (:`then`
        (`/Game/Blueprints/System/BP_SpaceGameState.AddDestroyedTarget` _asbp_space_game_state))
      (:`CastFailed`
        _))
    (`|ExecutionSequence`
      (:`then_0`
        (set `self.bAlive` false)
        (`self.OnAsteroidExplode` Location Direction)
        ;[1 1 1] Disable radar aiming trace block
        (`PrimitiveComponent.SetCollisionObjectType` (`self.GeometryCollection`) "ECC_Destructible"))
      (:`then_1`
        ;[1 1 1] Spawn effects
        (`SceneComponent.K2_SetWorldLocation` _explosionparticles Location false true)
        (`ActorComponent.Activate` _explosionparticles true))
      (:`then_2`
        (`TimelineComponent.PlayFromStart` (`self.ExplosionEmission`))))))

(fn `GetAsteroidLocation`
  (returns (Location :type "Vector Structure"))
  (return (`KismetSystemLibrary.GetComponentBounds` (`self.GeometryCollection`))))

(fn `GetAsteroidVelocity`
  (returns (Velocity :type "Vector Structure"))
  (bind _geometrycollection (`self.GeometryCollection`))
  (`PrimitiveComponent.GetPhysicsLinearVelocity` _geometrycollection (`|GetArrayItem` (`SceneComponent.GetAllSocketNames` _geometrycollection)))
  (return (`self.StartVelocityL`)))

(fn `GetExplosionMagnitude`
  (returns (Magnitude :type "Float (double-precision)"))
  (return (* (`|GetArrayItem` (`GeometryCollectionComponent.DamageThreshold` (`self.GeometryCollection`))) 10.0)))

(fn `GetExplosionRadius`
  (params (Divisor :type "Float (double-precision)" :default 1.0))
  (returns (Radius :type "Float (double-precision)"))
  (return (/ (`.SphereRadius` (`KismetSystemLibrary.GetComponentBounds` (`self.GeometryCollection`))) Divisor)))

(fn `IsAlive`
  (returns (bAlive :type Boolean))
  (return (`self.bAlive`)))

(fn `ProcessHit`
  (params (Point :type "Vector Structure") (Direction :type "Vector Structure"))
  (locals (PenetrationDist :type "Float (double-precision)"))
  (bind _location (`self.GetAsteroidLocation`))
  (`|ExecutionSequence`
    (:`then_0`
      (set `local.PenetrationDist` (`KismetMathLibrary.Sqrt` (- (`KismetMathLibrary.Square` (`KismetMathLibrary.VSize` (- _location Point))) (`KismetMathLibrary.Square` (`KismetMathLibrary.GetPointDistanceToLine` _location Point Direction))))))
    (:`then_1`
      (`SceneComponent.K2_SetWorldRotation` (`self.ExplosionParticles`) (`KismetMathLibrary.MakeRotFromX` Direction) false false))
    (:`then_2`
      (`self.Explode` (+ Point (* Direction (`local.PenetrationDist`))) Direction))))

(fn `SetEmissionScale`
  (params (Scale :type "Float (double-precision)") (Emission :type "Float (double-precision)") (Heat :type "Float (double-precision)"))
  (bind _asteroidmaterial (`self.AsteroidMaterial`))
  (`MaterialInstanceDynamic.SetScalarParameterValue` _asteroidmaterial "Glowing" Scale)
  (`MaterialInstanceDynamic.SetScalarParameterValue` _asteroidmaterial "Emisssive_Intencity" Emission)
  (`MaterialInstanceDynamic.SetScalarParameterValue` _asteroidmaterial "AdditiveHeat" Heat))

(fn `UserConstructionScript`)