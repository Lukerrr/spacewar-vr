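; Controller for a periscope that moves player control between the character pawn and a Periscope pawn.
; ActivatePeriscope caches the current pawn, possesses the periscope, notifies it and plays an enter sound.
; DeactivatePeriscope re-possesses the cached pawn, notifies the periscope and plays a leave sound.
; PowerOff, the right-button action and a debug Q key all trigger deactivation, but only while the periscope is possessed.
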(event EventPowerOff
  (if (Default|IsPossessed (Variables|Default|GetPeriscope))
    (CallFunction|DeactivatePeriscope)))

(event Input|ActionEvents|InputActionButtonRight_Action
  (params (Key :type Key%20Structure :default "None"))
  (:Pressed
    (if (Default|IsPossessed (Variables|Default|GetPeriscope))
      (CallFunction|DeactivatePeriscope))))

(event Input|KeyboardEvents|DebugKeyQ
  (params (Key :type Key%20Structure :default "None") (ActionValue :type Input%20Action%20Value%20Structure))
  (:Pressed
    (if (Default|IsPossessed (Variables|Default|GetPeriscope))
      (CallFunction|DeactivatePeriscope))))

(fn ConstructionScript)

(fn ActivatePeriscope
  (bind _returnvalue (Game|GetPlayerController 0))
  (bind _periscope (Variables|Default|GetPeriscope))
  (Variables|Default|SetCharacterPawn (Pawn|GetControlledPawn _returnvalue))
  (Pawn|Possess _returnvalue _periscope)
  (Default|OnPossessed _periscope)
  (Audio|PlaySound2D "/Game/ThirdParty/AFCore/Sound/Waves/Panel/Wave_Enter_Simulate.Wave_Enter_Simulate" 1.0 1.0 0.0 0 0))

(fn DeactivatePeriscope
  (Pawn|Possess (Game|GetPlayerController 0) (Variables|Default|GetCharacterPawn))
  (Default|OnUnpossessed (Variables|Default|GetPeriscope))
  (Audio|PlaySound2D "/Game/ThirdParty/AFCore/Sound/Waves/Panel/Wave_Leave_Simulate.Wave_Leave_Simulate" 1.0 1.0 0.0 0 0))