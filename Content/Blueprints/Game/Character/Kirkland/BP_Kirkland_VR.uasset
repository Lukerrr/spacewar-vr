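; BP_Kirkland_VR is the VR Blueprint for the Kirkland character, adding carried tools and pause menu control.
; On BeginPlay it hangs the flashlight and wrench child actors on separate hang components through each item's BPC_HangItemComponent.
; The Pause input toggles the menu on a BP_PauseMenu_Display, retrieved by casting the PauseDisplay child actor.
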(event `self.ReceiveBeginPlay`
  (`parent.ReceiveBeginPlay`)
  (`/Game/VRGK/Blueprints/Components/ItemHang/BPC_HangComponent.HangItem` (`self.BPC_HangComponent1`) (`self.GetComponentByClass` (`ChildActorComponent.ChildActor` (`self.Flashlight`)) "/Game/VRGK/Blueprints/Components/ItemHang/BPC_HangItemComponent.BPC_HangItemComponent_C"))
  (`/Game/VRGK/Blueprints/Components/ItemHang/BPC_HangComponent.HangItem` (`self.BPC_HangComponent`) (`self.GetComponentByClass` (`ChildActorComponent.ChildActor` (`self.Wrench`)) "/Game/VRGK/Blueprints/Components/ItemHang/BPC_HangItemComponent.BPC_HangItemComponent_C")))

(event `InputAction|Pause`
  (params (Key :type "Key Structure"))
  (:`Pressed`
    (`/Game/Blueprints/World/PauseMenu/BP_PauseMenu_Display.TogglePauseMenu` (`self.GetPauseDisplay`))))

(fn `GetPauseDisplay`
  (returns (PauseDisplay :type "/Game/Blueprints/World/PauseMenu/BP_PauseMenu_Display Object Reference"))
  (bind _asbp_pause_menu_display (cast `/Game/Blueprints/World/PauseMenu/BP_PauseMenu_Display` (`ChildActorComponent.ChildActor` (`self.PauseDisplay`)))
    (:`then`
      (return _asbp_pause_menu_display))
    (:`CastFailed`
      (return null))))

(fn `UserConstructionScript`
  (`parent.UserConstructionScript`))