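; Transient pawn that takes over the player during level transitions, showing a surrounding room and optional loading-screen widget that smoothly follows view rotation.
; TransitToLevel either quits or possesses the pawn, then unloads the current streamed level, loads the target and signals completion.
; Progress is estimated per stage by comparing the world's actor count to stored level sizes.
; With the loading screen, a timeline eases progress to 100% before finishing.
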(event `self.ReceiveTick`
  (params (DeltaSeconds :type "Float (single-precision)"))
  (bind _widgetroot (`self.WidgetRoot`))
  (bind _returnvalue (`KismetMathLibrary.Conv_IntToDouble` (`self.GetNumActorsLoaded`)))
  (if (`self.IsPossessed`)
    (`SceneComponent.K2_SetWorldRotation` _widgetroot (`KismetMathLibrary.RInterpTo` (`SceneComponent.K2_GetComponentRotation` _widgetroot) (`self.GetControlRotation`) (`GameplayStatics.GetWorldDeltaSeconds`) (`self.GuiRotationSpeed`)) false false))
  (`|ExecutionSequence`
    (:`then_0`
      (switch `/Game/Blueprints/Game/Character/TransientPawn/Enums/BPE_LevelTransitionStage` (`self.LevelTransitionStage`)
        (:`NewEnumerator0`
          (`self.SetTransitionPercentage` 100.0))
        (:`NewEnumerator1`
          (`self.SetTransitionPercentage` (`KismetMathLibrary.Lerp` 0.0 20.0 (/ _returnvalue (`KismetMathLibrary.Conv_IntToDouble` (`self.GetLevelSizeByType` (`self.OldLoadLevel`)))))))
        (:`NewEnumerator2`
          (`self.SetTransitionPercentage` (`KismetMathLibrary.Lerp` 20.0 (`self.LevelFinishingPercentage`) (/ _returnvalue (`KismetMathLibrary.Conv_IntToDouble` (`self.GetLevelSizeByType` (`self.NextLoadLevel`)))))))))))

(event `InputAxisKey|MouseX`
  (params (AxisValue :type "Float (single-precision)"))
  ;[1 1 1] Mouse rotation (DEBUG ONLY)
  (`self.AddControllerYawInput` AxisValue))

(event `OnPossessed`
  ;[1 1 1] Enable/disable HUD and fog on possess
  (`SceneComponent.SetVisibility` (`self.RoomRoot`) true true))

(event `InputAxisKey|MouseY`
  (params (AxisValue :type "Float (single-precision)"))
  ;[1 1 1] Mouse rotation (DEBUG ONLY)
  (`self.AddControllerPitchInput` (* AxisValue -1.0)))

(event `OnUnpossessed`
  ;[1 1 1] Enable/disable HUD and fog on possess
  (`SceneComponent.SetVisibility` (`self.Widget`) false false)
  (`SceneComponent.SetVisibility` (`self.RoomRoot`) false true))

(event `OnRequestTransit`
  (params (Level :type "/Game/Blueprints/Game/Character/TransientPawn/Enums/BPE_GameLevelType Enum" :default "NewEnumerator0") (bNeedsFinishing :type Boolean))
  ;[1 1 1] Transit to level
  ;;[1 1 1] Unload current level
  (set `self.LevelTransitionStage` "NewEnumerator1")
  (set `self.OldLoadLevel` (`self.NextLoadLevel`))
  (set `self.NextLoadLevel` Level)
  (`GameplayStatics.UnloadStreamLevelBySoftObjectPtr` (`self.GetLevelByType` (`self.OldLoadLevel`)))
  ;;[1 1 1] Load target level
  (set `self.LevelTransitionStage` "NewEnumerator2")
  (`GameplayStatics.LoadStreamLevelBySoftObjectPtr` (`self.GetLevelByType` (`self.NextLoadLevel`)) true true)
  (if bNeedsFinishing
    (set `self.LevelTransitionStage` "NewEnumerator3")
    (bind (_direction _percentagealpha) (`Timeline|Timeline_TransitFinish` :!via `PlayFromStart`)
      (:`Update`
        (`self.SetTransitionPercentage` (`KismetMathLibrary.Lerp` (`self.LevelFinishingPercentage`) 100.0 _percentagealpha)))
      (:`Finished`
        (`self.OnTransitFinished` :!label _label)
        (set `self.LevelTransitionStage` "NewEnumerator0")))
    (else
      (goto _label))))

(fn `GetGui`
  (returns (Gui :type "/Game/Blueprints/Widget/LoadingScreen/BP_LoadingScreen Object Reference"))
  (bind _asbp_loading_screen (cast `/Game/Blueprints/Widget/LoadingScreen/BP_LoadingScreen` (`WidgetComponent.GetWidget` (`self.Widget`)))
    (:`then`
      _)
    (:`CastFailed`
      _))
  (return _asbp_loading_screen))

(fn `GetLevelByType`
  (params (Type :type "/Game/Blueprints/Game/Character/TransientPawn/Enums/BPE_GameLevelType Enum" :default "NewEnumerator0"))
  (returns (Level :type "World Soft Object Reference"))
  (return (`BlueprintMapLibrary.Map_Find` (`self.LevelTypes`) Type)))

(fn `GetLevelSizeByType`
  (params (Type :type "/Game/Blueprints/Game/Character/TransientPawn/Enums/BPE_GameLevelType Enum" :default "NewEnumerator0"))
  (returns (Size :type Integer))
  (return (`BlueprintMapLibrary.Map_Find` (`self.LevelSizes`) Type)))

(fn `GetNumActorsLoaded`
  (returns (NumActors :type Integer))
  (bind _outactors (`GameplayStatics.GetAllActorsOfClass` "/Script/Engine.Actor"))
  (return (`KismetArrayLibrary.Array_Length` _outactors)))

(fn `IsPossessed`
  (returns (bPossessed :type Boolean))
  (return (`self.IsPlayerControlled`)))

(fn `SetTransitionPercentage`
  (params (Percentage :type "Float (double-precision)"))
  (`/Game/Blueprints/Widget/LoadingScreen/BP_LoadingScreen.SetLoadingPercent` (`self.GetGui`) Percentage))

(fn `TransitToLevel`
  (params (Level :type "/Game/Blueprints/Game/Character/TransientPawn/Enums/BPE_GameLevelType Enum" :default "NewEnumerator0") (bLoadingScreen :type Boolean))
  (if (`self.IsPossessed`)
    _
    (elif (`|EnumEquality` Level "NewEnumerator0")
      (`KismetSystemLibrary.QuitGame` (`GameplayStatics.GetPlayerController` 0) "Quit")
      (else
        (`SceneComponent.SetVisibility` (`self.Widget`) bLoadingScreen false)
        (`Controller.Possess` (`GameplayStatics.GetPlayerController` 0) self)
        (`self.OnPossessed`)
        (`self.OnRequestTransit` Level bLoadingScreen)))))

(fn `UserConstructionScript`)