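; Debug pawn for pointing at widgets, dragging physics objects and testing electric panel hits.
; A WidgetInteraction component follows control rotation and supplies the forward vector for line traces and the grab target.
; Left mouse both clicks widgets and grabs through a PhysicsHandle at the traced distance, reapplying game-only input as an engine bug workaround.
; A debug key traces a short range to simulate a wrench hit on BP_ElectricPanel.
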(event EventUnpossessed
  (params (OldController :type Controller%20Object%20Reference))
  (Physics|Components|PhysicsHandle|ReleaseComponent (Variables|Default|GetPhysicsHandle)))

(event EventTick
  (params (DeltaSeconds :type Float%20%28single-precision%29))
  ;[1 1 1] Move widget pointer
  (Transformation|SetWorldRotation (Variables|Default|GetWidgetInteraction) (Pawn|GetControlRotation :!class /Script/Engine.Pawn) false false)
  ;[1 1 1] Move grabbed object
  (Physics|Components|PhysicsHandle|SetTargetLocation (Variables|Default|GetPhysicsHandle) (CallFunction|GetPointatForward (Variables|Default|GetGrabbedComponentDistance))))

(event Input|KeyboardEvents|DebugKeyR
  (params (Key :type Key%20Structure :default "None") (ActionValue :type Input%20Action%20Value%20Structure))
  (:Pressed
    (bind _outhit (Collision|LineTraceByChannel (Transformation|GetActorLocation) (CallFunction|GetPointatForward 2e+02) "TraceTypeQuery1" false 0 "None"))
    (bind _asbp_electric_panel (Utilities|Casting|CastToBP_ElectricPanel (.hitactor _outhit)))
    (Default|OnWrenchHit _asbp_electric_panel 2e+02 (.location _outhit))))

(event Input|MouseEvents|LeftMouseButton
  (params (Key :type Key%20Structure :default "None"))
  (bind _widgetinteraction (Variables|Default|GetWidgetInteraction))
  ;[1 1 1] Widget interactions with pointer
  (:Pressed
    (Class|WidgetInteractionComponent|PressPointerKey _widgetinteraction "LeftMouseButton")
    ;;[1 0 0] FIXME: W/a for UE-166377
    (Input|SetInputModeGameOnly (Game|GetPlayerController 0) false)
    ;[1 1 1] Grabbing physical objects
    (|EnableGrab))
  (:Released
    (Class|WidgetInteractionComponent|ReleasePointerKey _widgetinteraction "LeftMouseButton")
    (Input|SetInputModeGameOnly (Game|GetPlayerController 0) false)
    (|ReleaseGrab)))

(fn ConstructionScript)

(fn GetPointatForward
  (params (Distance :type Float%20%28double-precision%29))
  (return (+ (Transformation|GetActorLocation) (* (Math|Vector|GetForwardVector (Variables|Default|GetWidgetInteraction)) Distance))))